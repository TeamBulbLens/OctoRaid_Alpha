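; BP_RespawnAreaN is a respawn area actor that supplies a randomized ground-level respawn transform within its Box component.
; GetRespawnPoint picks random points in the box bounds and line-traces downward against WorldStatic objects.
; It returns the hit location with zero rotation and unit scale, without checking whether the trace hit.
; The event graph and construction script contain no logic.
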(event EventBeginPlay)

(event Collision|EventActorBeginOverlap
  (params (OtherActor :type Actor%20Object%20Reference)))

(event EventTick
  (params (DeltaSeconds :type Float%20%28single-precision%29)))

(fn ConstructionScript)

(fn GetRespawnPoint
  (bind _returnvalue (Transformation|GetActorLocation))
  (bind _box (Variables|Default|GetBox))
  (bind _returnvalue_2 (Components|Box|GetScaledBoxExtent _box))
  (bind _returnvalue_3 (Math|Random|RandomPointinBoundingBox _returnvalue _returnvalue_2))
  (bind _outhit (Collision|LineTraceForObjects _returnvalue_3 (+ _returnvalue_3 (* (Math|Vector|VectorDown) 1e+03)) (Utilities|Array|MakeArray "ObjectTypeQuery1") false 0 "None"))
  (if true
    (return (Math|Transform|MakeTransform (+ (.Location (Collision|BreakHitResult _outhit)) "0, 0,0.000000") "0, 0, 0" "1,1.000000,1"))))