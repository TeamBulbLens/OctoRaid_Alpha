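; BP_RespawnArea is a box volume that supplies respawn transforms and reports whether it is safely above the water.
; GetRespawnPoint line-traces down from random points in the box against WorldStatic, lifts the hit slightly and yaws it toward the world origin.
; A failed trace falls back to the actor's location.
; Avaliable compares the box's lower portion with the higher of BP_MainGS's blue and dead water heights plus a margin.
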(fn ConstructionScript)

(fn GetRespawnPoint
  (bind _returnvalue (Transformation|GetActorLocation))
  (bind _returnvalue_2 (Transformation|GetActorLocation))
  (bind _box (Variables|Default|GetBox))
  (bind _returnvalue_3 (Components|Box|GetScaledBoxExtent _box))
  (bind _returnvalue_4 (Math|Random|RandomPointinBoundingBox _returnvalue_2 _returnvalue_3))
  ;[1 1 1] box 볼륨 내 랜덤 위치를 리턴
  (bind (_outhit _returnvalue_5) (Collision|LineTraceForObjects _returnvalue_4 (+ _returnvalue_4 (* (Math|Vector|VectorDown) 1e+03)) (Utilities|Array|MakeArray "ObjectTypeQuery1") false 0 "None"))
  (if _returnvalue_5
    (return (Math|Transform|MakeTransform (+ (.Location (Collision|BreakHitResult _outhit)) "0,0.000000,100.000000") (Math|Rotator|MakeRotator 0.0 0.0 (.yaw (Math|Rotator|FindLookatRotation (+ (.Location (Collision|BreakHitResult _outhit)) "0,0.000000,100.000000") (Math|Vector|MakeVector 0.0 0.0 0.0)))) "1,1,1"))
    (else
      ;;[1 1 1] 랜덤 지점 가져오기가 실패할 경우 기본값으로 액터 가운데 지점 가져오기
      (return (Math|Transform|MakeTransform _returnvalue (Math|Rotator|MakeRotator 0.0 0.0 (.yaw (Math|Rotator|FindLookatRotation _returnvalue (Math|Vector|MakeVector 0.0 0.0 0.0)))) "1,1,1")))))

(fn Avaliable
  (bind _asbp_main_gs (Utilities|Casting|CastToBP_MainGS (Game|GetGameState))
    (:then
      (return (> (- (.z (Transformation|GetActorLocation)) (/ (.z (Components|Box|GetScaledBoxExtent (Variables|Default|GetBox))) 2.0)) (+ (Math|Float|Max(Float) (Variables|/Game/Blueprints/System/Main/BP_MainGS.BP_MainGS_C|GetBlueWaterHeight _asbp_main_gs) (Variables|/Game/Blueprints/System/Main/BP_MainGS.BP_MainGS_C|GetDeadWaterHeight _asbp_main_gs)) (Variables|Default|GetWater감지간격)))))
    (:CastFailed
      (return false))))